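; BP_CMiku is a Miku Blueprint that prepares its mesh materials for a controllable light direction.
; The construction script wraps each mesh material in a dynamic instance, stores it in DynamicMaterials and uses the returned array index as its material slot.
; It then pushes the Light variable into the LightDirection vector parameter across all materials.
; The event graph holds only empty events, so nothing updates at runtime.
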(event EventBeginPlay)

(event Collision|EventActorBeginOverlap
  (params (OtherActor :type Actor%20Object%20Reference)))

(event EventTick
  (params (DeltaSeconds :type Float%20%28single-precision%29)))

(fn ConstructionScript
  (for _array_element (Rendering|Material|GetMaterials (Variables|Character|GetMesh))
    (bind _returnvalue (Rendering|Material|CreateDynamicMaterialInstance _array_element "None" :!class /Script/Engine.KismetMaterialLibrary))
    (bind _returnvalue_2 (Utilities|Array|Add (Variables|Default|GetDynamicMaterials) _returnvalue))
    (Rendering|Material|SetMaterial (Variables|Character|GetMesh) _returnvalue_2 _returnvalue))
  (Rendering|Material|SetVectorParameterValueonMaterials (Variables|Character|GetMesh) "LightDirection" (Variables|Default|GetLight)))