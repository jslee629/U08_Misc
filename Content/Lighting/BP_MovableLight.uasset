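; BP_MovableLight is an actor, filed under Lighting, that moves in a continuous horizontal circle around its placed position.
; BeginPlay stores the starting location as the orbit center.
; Each Tick, sine and cosine of game time drive a fixed-radius X/Y offset from that center, with height unchanged and no sweep.
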(event EventBeginPlay
  (Variables|Default|SetStart (Transformation|GetActorLocation)))

(event EventTick
  (params (DeltaSeconds :type Float%20%28single-precision%29))
  (bind _returnvalue (Utilities|Time|GetTimeSeconds))
  (Transformation|SetActorLocation (+ (Variables|Default|GetStart) (Math|Vector|MakeVector (* 300 (Math|Trig|Sin(Radians) _returnvalue)) (* 300 (Math|Trig|Cos(Radians) _returnvalue)) 0.0)) false false))

(fn ConstructionScript)